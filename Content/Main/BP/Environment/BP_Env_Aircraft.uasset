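; Environment aircraft actor with an optional floating movement, run once from BeginPlay when IsFloating is set.
; FloatingMovement toggles IsUp to pick a one-unit Y direction, then applies a lerped vector as a world offset.
; The lerp alpha is fixed at zero, so the offset equals the actor's current location and the chosen direction has no effect.
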(event EventBeginPlay
  (if (Variables|Default|GetisFloating)
    (Utilities|FloatingMovement)))

(event Collision|EventActorBeginOverlap
  (params (OtherActor :type Actor%20Object%20Reference)))

(fn ConstructionScript)