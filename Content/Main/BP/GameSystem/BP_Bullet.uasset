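; Bullet actor that shows an impact effect and reports damage to shootable targets.
; When the bullet mesh hits anything other than player 0's character, it swaps the laser particles for an explosion and sets its life duration.
; It then casts the hit actor to BP_Target and passes Damage to OnBeingShot.
; An unconnected debug branch remains in the event graph.
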(event OnComponentHit(BulletMesh)
  (params (HitComponent :type Primitive%20Component%20Object%20Reference) (OtherActor :type Actor%20Object%20Reference) (OtherComp :type Primitive%20Component%20Object%20Reference) (NormalImpulse :type Vector :default "0, 0, 0") (Hit :type Hit%20Result%20Structure%20%28by%20ref%29))
  (if (!= OtherActor (Game|GetPlayerCharacter 0))
    (Components|Activation|Deactivate (Variables|Default|GetPS_Laser))
    (Components|Activation|Activate (Variables|Default|GetPS_Explosion) false)
    (Variables|Default|SetLifeDuration 5.0)
    (bind _asbp_target (Utilities|Casting|CastToBP_Target OtherActor))
    (Default|OnBeingShot _asbp_target (Variables|Default|GetDamage))))

(event EventBeginPlay)

(event Collision|EventActorBeginOverlap
  (params (OtherActor :type Actor%20Object%20Reference)))

(fn ConstructionScript)