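; BP_Target is a shootable target actor that tracks health, reacts visually to hits and destroys itself when health runs out.
; OnBeingShot subtracts damage, then either calls Die or activates a hit particle and briefly swaps the mesh to a hit material, restoring the one cached at BeginPlay and later deactivating the particle.
; Die reuses that particle component with a death template, then destroys the actor after a zero-length delay.
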(event Custom|OnBeingShot
  (params (Damage :type Integer))
  (bind _output_get (Variables|Default|SetHealth (- (Variables|Default|GetHealth) Damage)))
  (if (<= _output_get 0)
    (CallFunction|Die)
    (else
      (Components|Activation|Activate (Variables|Default|GetPS_BeingShot) false)
      (Rendering|Material|SetMaterial (Variables|Default|GetSM) 0 (Variables|Default|GetMat_BeingHit))
      (Utilities|FlowControl|Delay 0.33)
      (Rendering|Material|SetMaterial (Variables|Default|GetSM) 0 (Variables|Default|GetMat_Normal))
      (Utilities|FlowControl|Delay 4.0)
      (Components|Activation|Deactivate (Variables|Default|GetPS_BeingShot)))))

(event Custom|Die
  (Effects|Components|ParticleSystem|SetTemplate (Variables|Default|GetPS_BeingShot) (Variables|Default|GetPS_Die))
  (Components|Activation|Activate (Variables|Default|GetPS_BeingShot) false)
  (Utilities|FlowControl|Delay 0.0)
  (Actor|DestroyActor))

(event EventBeginPlay
  (Variables|Default|SetMat_Normal (Utilities|Array|Get(acopy) (Rendering|Material|GetMaterials (Variables|Default|GetSM)))))

(event Collision|EventActorBeginOverlap
  (params (OtherActor :type Actor%20Object%20Reference)))

(event EventTick
  (params (DeltaSeconds :type Float%20%28single-precision%29)))

(fn ConstructionScript)