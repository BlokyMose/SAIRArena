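; BP_Craft_Zero is a craft Blueprint that handles the visual feedback for movement and thrusting.
; The MovingCallback event activates or deactivates the left and right turbo particle components as the craft starts or stops moving.
; The Thrusting event swaps both particle templates between throttle and turbo effects and toggles the PPThrusting post-process to match.
; Tick, BeginPlay and overlap events are disabled stubs, so all logic here is event-driven.
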(event EventBeginPlay
  (|CallParentFunction) ; This node is disabled and will not be called.\nDrag off pins to build functionality.
)

(event Collision|EventActorBeginOverlap
  (params (OtherActor :type Actor%20Object%20Reference))
  (|CallParentFunction OtherActor) ; This node is disabled and will not be called.\nDrag off pins to build functionality.
)

(event EventTick
  (params (DeltaSeconds :type Float%20%28single-precision%29))
  (|CallParentFunction DeltaSeconds) ; This node is disabled and will not be called.\nDrag off pins to build functionality.
)

(event EventThrusting
  (params (BPbIsThrusting :type Boolean))
  (if BPbIsThrusting
    (Effects|Components|ParticleSystem|SetTemplate (Variables|Default|GetTurboRight) "/Game/Main/BP/Particle/PS_Turbo.PS_Turbo")
    (Effects|Components|ParticleSystem|SetTemplate (Variables|Default|GetTurboLeft) "/Game/Main/BP/Particle/PS_Turbo.PS_Turbo")
    (Variables|/Script/Engine.PostProcessComponent|SetbEnabled (Variables|Default|GetPP_Thrusting) true)
    (else
      (Effects|Components|ParticleSystem|SetTemplate (Variables|Default|GetTurboRight) "/Game/Main/BP/Particle/PS_Throttle.PS_Throttle")
      (Effects|Components|ParticleSystem|SetTemplate (Variables|Default|GetTurboLeft) "/Game/Main/BP/Particle/PS_Throttle.PS_Throttle")
      (Variables|/Script/Engine.PostProcessComponent|SetbEnabled (Variables|Default|GetPP_Thrusting) false))))

(event EventMovingCallback
  (params (isMoving :type Boolean))
  (if isMoving
    (Components|Activation|Activate (Variables|Default|GetTurboRight) false)
    (Components|Activation|Activate (Variables|Default|GetTurboLeft) false)
    (else
      (Components|Activation|Deactivate (Variables|Default|GetTurboRight))
      (Components|Activation|Deactivate (Variables|Default|GetTurboLeft)))))

(fn ConstructionScript
  (|CallParentFunction))