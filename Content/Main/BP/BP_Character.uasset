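; BP_Character is a character Blueprint that handles HUD, health display and overlap interaction, with forward tracing deferred to its parent.
; On BeginPlay it adds crosshair and HUD widgets, then pushes SAIRHealth values to the HUD, repeating this on any damage.
; Mesh overlaps send OnInteractMessage to the other actor, passing itself.
; TraceForward only calls the parent implementation; a Blueprint camera line trace remains unconnected.
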(event OnComponentBeginOverlap(MeshCom)
  (params (OverlappedComponent :type Primitive%20Component%20Object%20Reference) (OtherActor :type Actor%20Object%20Reference) (OtherComp :type Primitive%20Component%20Object%20Reference) (OtherBodyIndex :type Integer) (bFromSweep :type Boolean) (SweepResult :type Hit%20Result%20Structure%20%28by%20ref%29))
  ;[1 1 1] Overlap
  (Class|InterfaceInteract|OnInteract(Message) OtherActor self))

(event EventBeginPlay
  ;[0.5521 1 0.6993] UI
  (bind _returnvalue (UserInterface|CreateWidget "/Game/Main/BP/UI/WBP_Crosshair.WBP_Crosshair_C"))
  (UserInterface|Viewport|AddtoViewport _returnvalue 0)
  (bind _returnvalue_2 (UserInterface|CreateWidget "/Game/Main/BP/UI/WBP_HUD.WBP_HUD_C"))
  (bind _output_get (Variables|Default|SetHUDRef _returnvalue_2))
  (UserInterface|Viewport|AddtoViewport _output_get 0)
  (CallFunction|UpdateProgHealthBar))

(event EventTraceForward
  ;[1 1 1] Evend Trace Combi
  (|CallParentFunction))

(event Game|Damage|EventAnyDamage
  (params (Damage :type Float%20%28single-precision%29) (DamageType :type Damage%20Type%20Object%20Reference) (InstigatedBy :type Controller%20Object%20Reference) (DamageCauser :type Actor%20Object%20Reference))
  ;[0.1237 0.4719 0.1822] Health
  (CallFunction|UpdateProgHealthBar))

(event Input|ActionEvents|InputActionInteract
  (params (Key :type Key%20Structure :default "None"))
  ;[1 1 1] Input Trace
)

(fn ConstructionScript)

(fn UpdateProgHealthBar
  (bind _sair_health (Variables|Default|GetSAIR_Health))
  (Utilities|IsValid (Variables|Default|GetSAIR_Health)
    (:Is%20Valid
      (Default|UpdateHealth (Variables|Default|GetHUDRef) (Variables|/Script/SAIRArena.SAIR_HealthComponent|GetHealth _sair_health) (Variables|/Script/SAIRArena.SAIR_HealthComponent|GetDefaultHealth _sair_health)))))