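; BP_InteractableBase is an interactable object base that changes its cube's color when it gains or loses focus.
; On BeginPlay it creates a dynamic material instance on the Cube and caches its Color parameter as the default.
; StartFocus and EndFocus swap that parameter between the focus color and the cached default, each also printing a debug string.
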(event EventBeginPlay
  ;[1 0 0.111] BeginPlay
  (bind _returnvalue (Rendering|Material|CreateDynamicMaterialInstance (Variables|Default|GetCube) 0 0 "None" :!class /Script/Engine.PrimitiveComponent))
  (bind _output_get (Variables|Default|SetMaterialInstance _returnvalue))
  (bind _returnvalue_2 (Rendering|Material|GetVectorParameterValue _output_get "Color" :!class /Script/Engine.MaterialInstanceDynamic))
  (Variables|Default|SetDefaultColor _returnvalue_2))

(event EventStartFocus
  ;[1 0.6555 0] Focus/Unfocused
  (Development|PrintString "Hello")
  (Rendering|Material|SetVectorParameterValue (Variables|Default|GetMaterialInstance) "Color" (Variables|Default|GetFocusColor) :!class /Script/Engine.MaterialInstanceDynamic))

(event EventEndFocus
  ;[1 0.6555 0] Focus/Unfocused
  (Development|PrintString "NOPE")
  (Rendering|Material|SetVectorParameterValue (Variables|Default|GetMaterialInstance) "Color" (Variables|Default|GetDefaultColor) :!class /Script/Engine.MaterialInstanceDynamic))

(fn ConstructionScript)