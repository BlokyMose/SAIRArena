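; BP_ScrollingComponent is an actor component that scrolls its owning actor along while an Endless-mode level is playing.
; On BeginPlay it caches the level manager found through a Blueprint library lookup.
; Each Tick, while that manager reports playing, it scales the owner's forward vector by the manager's LevelSpeed and delta time.
; The result is applied as a local-space offset without sweep, although the forward vector is in world space.
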(event EventTick
  (params (DeltaSeconds :type Float%20%28single-precision%29))
  (bind _levelmanagerref (Variables|Default|GetLevelManagerRef))
  (Utilities|IsValid _levelmanagerref
    (:Is%20Valid
      (if (Variables|/Game/Main/Endless/BP_Endless/Game/BP_LevelManager.BP_LevelManager_C|GetbIsPlaying _levelmanagerref)
        (Variables|Default|SetDeltaSeconds DeltaSeconds)
        (bind _output_get (Variables|Default|SetMovement (* (* (Transformation|GetActorForwardVector (Components|GetOwner)) (Variables|/Game/Main/Endless/BP_Endless/Game/BP_LevelManager.BP_LevelManager_C|GetLevelSpeed (Variables|Default|GetLevelManagerRef))) (Variables|Default|GetDeltaSeconds))))
        (Transformation|AddActorLocalOffset (Components|GetOwner) _output_get false false)))))

(event EventBeginPlay
  (bind (_levelmanager _levelmanagerfound) (CallFunction|GetLevelManager))
  (if _levelmanagerfound
    (Variables|Default|SetLevelManagerRef _levelmanager)))