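; Endless-mode floor spawner that keeps a continuous strip of ground tiles by recycling a fixed set of actors.
; On BeginPlay it spawns tiles through the parent SpawnActor, measures tile length from the first one's bounds, and lines the rest up along X.
; When a spawned tile hits bounds, it is moved one tile length past the current RearTile and becomes the new RearTile.
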(event EventBeginPlay
  (for _index (range 0 (Variables|Default|GetActorRequiredCount))
    (if (== _index 0)
      (bind _returnvalue (CallFunction|SpawnActor))
      (Variables|Default|SetRearTile _returnvalue)
      (Variables|Default|SetTileSize (* (.x (.BoxExtent (Collision|GetActorBounds _returnvalue false false))) 2.0))
      (Transformation|SetActorLocationAndRotation (Variables|Default|GetRearTile) (Transformation|GetActorLocation))
      (else
        (bind _returnvalue_2 (CallFunction|SpawnActor))
        (Transformation|SetActorLocation _returnvalue_2 (Math|Vector|MakeVector (+ (Variables|Default|GetTileSize) (.x (Transformation|GetActorLocation (Variables|Default|GetRearTile)))) (.y (Transformation|GetActorLocation (Variables|Default|GetRearTile))) 0.0) false false)
        (Variables|Default|SetRearTile _returnvalue_2)))))

(event EventSpawnedActorHitBounds
  (params (OutOfBoundActor :type Actor%20Object%20Reference))
  (Transformation|SetActorLocation OutOfBoundActor (Math|Vector|MakeVector (+ (.x (Transformation|GetActorLocation (Variables|Default|GetRearTile))) (Variables|Default|GetTileSize)) (.y (Transformation|GetActorLocation (Variables|Default|GetRearTile))) (.z (Transformation|GetActorLocation (Variables|Default|GetRearTile)))) false false)
  (Variables|Default|SetRearTile OutOfBoundActor))

(fn ConstructionScript
  (|CallParentFunction))

(fn SpawnActor
  (bind _returnvalue (|CallParentFunction))
  (return _returnvalue))