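; BP_ER_PawnBase is the base player pawn for an endless runner, moving sideways between lanes.
; On begin play it reads lane count and width from the level manager, starts in the middle lane and finds the camera tagged EndCam.
; MoveRight axis input drives timelines that lerp Y one lane over, guarded by edge checks and a Moving flag.
; HitObstacle blends the view to the end camera and hides the player.
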(event EventBeginPlay
  (CallFunction|Initialize))

(event Input|AxisEvents|InputAxisMoveRight
  (params (AxisValue :type Float%20%28single-precision%29))
  (bind _returnvalue (Transformation|GetActorLocation))
  (bind _returnvalue_2 (Transformation|GetActorLocation))
  (if (Variables|/Game/Main/Endless/BP_Endless/Game/BP_LevelManager.BP_LevelManager_C|GetbIsPlaying (Variables|Default|GetLevelManagerRef))
    (if (== AxisValue -1.0)
      ;[1 1 1] Press Left whilst in the most Left
      (if (not (<= (Variables|Default|GetCurrentLane) 1))
        (if (not (Variables|Default|GetMoving))
          (Variables|Default|SetMoving true)
          (Variables|Default|SetTargetPosition (- (.y (Transformation|GetActorLocation)) (Variables|Default|GetLaneWidth)))
          (bind _move (Timeline|MoveLeft PlayFromStart)
            (:Update
              (Transformation|SetActorLocation (Math|Vector|MakeVector (.x _returnvalue_2) (Math|Float|Lerp (.y _returnvalue_2) (Variables|Default|GetTargetPosition) _move) (.z _returnvalue_2)) false false))
            (:Finished
              (Variables|Default|SetMoving false)
              (Math|Integer|DecrementInt (Variables|Default|GetCurrentLane))))))
      (elif (== AxisValue 1.0)
        (if (not (== (Variables|/Game/Main/Endless/BP_Endless/Game/BP_LevelManager.BP_LevelManager_C|GetNumberOfLanes (Variables|Default|GetLevelManagerRef)) (Variables|Default|GetCurrentLane)))
          (if (not (Variables|Default|GetMoving))
            (Variables|Default|SetMoving true)
            (Variables|Default|SetTargetPosition (+ (Variables|Default|GetLaneWidth) (.y (Transformation|GetActorLocation))))
            (bind _move_2 (Timeline|MoveRight PlayFromStart)
              (:Update
                (Transformation|SetActorLocation (Math|Vector|MakeVector (.x _returnvalue) (Math|Float|Lerp (.y _returnvalue) (Variables|Default|GetTargetPosition) _move_2) (.z _returnvalue)) false false))
              (:Finished
                (Variables|Default|SetMoving false)
                (Math|Integer|IncrementInt (Variables|Default|GetCurrentLane))))))))))

(fn ConstructionScript)

(fn Initialize
  (bind (_levelmanager _levelmanagerfound) (CallFunction|GetLevelManager))
  (if _levelmanagerfound
    (Variables|Default|SetLevelManagerRef _levelmanager)
    (Variables|Default|SetCurrentLane (+ (/ (Variables|/Game/Main/Endless/BP_Endless/Game/BP_LevelManager.BP_LevelManager_C|GetNumberOfLanes (Variables|Default|GetLevelManagerRef)) 2) 1))
    (Variables|Default|SetLaneWidth (Variables|/Game/Main/Endless/BP_Endless/Game/BP_LevelManager.BP_LevelManager_C|GetLaneWidth (Variables|Default|GetLevelManagerRef)))
    (bind _outactors (Actor|GetAllActorswithTag "EndCam"))
    (bind _output_get (Variables|Default|SetEndCamRef (Utilities|Array|Get(acopy) _outactors)))
    (Development|PrintString (Utilities|GetObjectName _output_get))
    (else
      (Development|PrintString "error no level man"))))

(fn HitObstacle
  (Game|Player|SetViewTargetwithBlend (Game|GetPlayerController 0) (Variables|Default|GetEndCamRef) 1.0 "VTBlend_Linear" 0.0 false)
  (Rendering|ToggleVisibility (Variables|Default|GetPlayer) false))